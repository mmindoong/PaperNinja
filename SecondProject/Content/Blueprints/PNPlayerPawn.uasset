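; Player pawn Blueprint with camera-relative movement, look controls, sprinting and a coin counter.
; Move and look axes drive movement input and controller rotation, while Sprint switches max walk speed between walk and sprint values.
; The first damage received prints a death message, disables movement and sets a short life span.
; AddCoin and GetNumOfCoins manage the coin total, with the C key adding coins as an apparent debug shortcut.
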(event `self.ReceiveBeginPlay`
  (set `CharacterMovementComponent.MaxWalkSpeed` (`self.GroundWalkSpeed`) (`self.CharacterMovement`)))

(event `InputAxis|MoveForward`
  (params (AxisValue :type "Float (single-precision)"))
  (`self.AddMovementInput` (`SceneComponent.GetForwardVector` (`self.Camera`)) AxisValue))

(event `self.ReceiveAnyDamage`
  (params (Damage :type "Float (single-precision)") (DamageType :type "DamageType Object Reference") (InstigatedBy :type "Controller Object Reference") (DamageCauser :type "Actor Object Reference"))
  (`/Engine/EditorBlueprintResources/StandardMacros.DoOnce` false ; AnyDamage가 한번만 실행
    (:`Completed`
      (`KismetSystemLibrary.PrintString` "Died" true true (struct :`R` 1.0 :`G` 0.00565 :`A` 1.0) 5.0)
      (`CharacterMovementComponent.DisableMovement` (`self.CharacterMovement`)) ; 쓰러지는 액션
      (`self.SetLifeSpan` 5.0))))

(event `InputAction|Sprint`
  (params (Key :type "Key Structure"))
  (bind _charactermovement (`self.CharacterMovement`))
  (:`Pressed`
    (set `CharacterMovementComponent.MaxWalkSpeed` (`self.GroundSprintSpeed`) _charactermovement))
  (:`Released`
    (set `CharacterMovementComponent.MaxWalkSpeed` (`self.GroundWalkSpeed`) _charactermovement)))

(event `Key|C`
  (params (Key :type "Key Structure"))
  (:`Pressed`
    (bind _aspnplayer_pawn (cast `/Game/Blueprints/PNPlayerPawn` (`GameplayStatics.GetPlayerPawn` 0)))
    (`self.AddCoin` _aspnplayer_pawn 5)))

(event `InputAxis|MoveRight`
  (params (AxisValue :type "Float (single-precision)"))
  (`self.AddMovementInput` (`SceneComponent.GetRightVector` (`self.Camera`)) AxisValue))

(event `InputAxis|LookUp`
  (params (AxisValue :type "Float (single-precision)"))
  (`self.AddControllerPitchInput` AxisValue))

(event `InputAxis|LookRight`
  (params (AxisValue :type "Float (single-precision)"))
  (`self.AddControllerYawInput` AxisValue))

(fn `AddCoin`
  (params (Num :type Integer))
  (set `self.NumOfCoins` (+ (`self.NumOfCoins`) Num)) ; c키->num=num+1;print(num)
)

(fn `GetNumOfCoins`
  (returns (ReturnValue :type Integer))
  (return (`self.NumOfCoins`)))

(fn `UserConstructionScript`)